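; Actor that slides in a straight line along relative Y between two hardcoded points, likely as a box spawned by other logic.
; On BeginPlay, the MoveBox timeline plays at a rate of 1/TimeBox, so TimeBox controls travel time.
; Each update lerps the relative location, with X and Z held constant.
; Unwired leftover nodes for spawning a cube mesh, rotating and offsetting never run.
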(event EventBeginPlay
  (Components|Timeline|SetPlayRate (Variables|Default|GetMoveBox) (/ 1.0 (Variables|Default|GetTimeBox)))
  (bind _newtrack_2 (Timeline|MoveBox Play)
    (:Update
      (Transformation|SetActorRelativeLocation (Math|Vector|MakeVector -164.0 (Math|Float|Lerp 343.0 -127.0 _newtrack_2) 9e+01)))))

(event Collision|EventActorBeginOverlap
  (params (OtherActor :type Actor%20Object%20Reference)))

(event EventTick
  (params (DeltaSeconds :type Float%20%28single-precision%29)))

(fn ConstructionScript)